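; Food Fighters game mode that creates local players at BeginPlay, each with its own HUD widget added to that player's screen.
; Players one and two are always created.
; A switch on PlayerCount resets start-closed DoOnce nodes, which chain creation of the third player, then the fourth, after player two so only the selected count spawns.
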(event EventBeginPlay
  (bind _returnvalue (Class|GameplayStatics|CreatePlayer 0))
  (bind _returnvalue_2 (UserInterface|CreateWidget "/Game/Blueprints/UI/HUDP1.HUDP1_C" _returnvalue))
  (UserInterface|Viewport|AddtoPlayerScreen _returnvalue_2)
  (Utilities|FlowControl|Sequence
    (:then_0
      (switch Utilities|FlowControl|Switch|SwitchonE_NumberOfPlayers (Variables|Default|GetplayerCount)
        (:NewEnumerator1
          (goto _label Reset))
        (:NewEnumerator2
          (Utilities|FlowControl|Sequence
            (:then_0
              (goto _label Reset))
            (:then_1
              (goto _label_2 Reset))))))
    (:then_1
      (bind _returnvalue_3 (Class|GameplayStatics|CreatePlayer 1))
      (bind _returnvalue_4 (UserInterface|CreateWidget "/Game/Blueprints/UI/HUDP2.HUDP2_C" _returnvalue_3))
      (UserInterface|Viewport|AddtoPlayerScreen _returnvalue_4)
      (Utilities|FlowControl|DoOnce true :!label _label
        (:Completed
          (bind _returnvalue_5 (Class|GameplayStatics|CreatePlayer 2))
          (bind _returnvalue_6 (UserInterface|CreateWidget "/Game/Blueprints/UI/HUDP3.HUDP3_C" _returnvalue_5))
          (UserInterface|Viewport|AddtoPlayerScreen _returnvalue_6)
          (Utilities|FlowControl|DoOnce true :!label _label_2
            (:Completed
              (bind _returnvalue_7 (Class|GameplayStatics|CreatePlayer 3))
              (bind _returnvalue_8 (UserInterface|CreateWidget "/Game/Blueprints/UI/HUDP4.HUDP4_C" _returnvalue_7))
              (UserInterface|Viewport|AddtoPlayerScreen _returnvalue_8))))))))

(fn ConstructionScript)