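; StandardProjectile is a projectile actor that moves through a ProjectileMovement component and destroys itself when it meets the floor.
; The construction script copies the InitialSpeed variable into the movement component and makes Skeleton its updated component.
; Hit checks the other component for the Floor tag, while ActorBeginOverlap checks the other actor.
; An unconnected "Plan B" impulse on the spine_01 bone never runs.
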(event Collision|EventActorBeginOverlap
  (params (OtherActor :type Actor%20Object%20Reference))
  (if (Actor|ActorHasTag OtherActor "Floor")
    (Actor|DestroyActor)))

(event Collision|EventHit
  (params (MyComp :type Primitive%20Component%20Object%20Reference) (Other :type Actor%20Object%20Reference) (OtherComp :type Primitive%20Component%20Object%20Reference) (bSelfMoved :type Boolean) (HitLocation :type Vector :default "0, 0, 0") (HitNormal :type Vector :default "0, 0, 0") (NormalImpulse :type Vector :default "0, 0, 0") (Hit :type Hit%20Result%20Structure%20%28by%20ref%29))
  ;[1 1 1] Destroy on contact with floor
  (if (Components|ComponentHasTag OtherComp "Floor")
    (Actor|DestroyActor)))

(fn ConstructionScript
  (bind _projectilemovement (Variables|Default|GetProjectileMovement))
  (Variables|/Script/Engine.ProjectileMovementComponent|SetInitialSpeed _projectilemovement (Variables|Default|GetinitialSpeed))
  (Components|Movement|SetUpdatedComponent _projectilemovement (Variables|Default|GetSkeleton)))